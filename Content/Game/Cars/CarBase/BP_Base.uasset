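; BP_Base is a base car pawn Blueprint that maps touch controls to inherited driving actions and handles headlight and dust effects.
; The primary thumbstick drives steering, throttle and brake with brake start/stop tracking, while the secondary looks around.
; Enhanced Input and touch headlight events share one FlipFlop that toggles both lights.
; A looping timer polls speed and arcade ground control to switch two sand dust effects, avoiding Tick.
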(event Custom|CheckVFX
  (if (and (> (Math|Vector|VectorLength (Transformation|GetVelocity)) 2e+01) (Class|MetalCarBase|CanUseArcadeGroundControl))
    (Components|Activation|Activate (Variables|Default|GetSandDust) false)
    (else
      (Components|Activation|Deactivate (Variables|Default|GetSandDust)))))

(event Input|EnhancedActionEvents|EnhancedInputActionIA_Headlights
  (params (ActionValue :type Boolean) (ElapsedSeconds :type Float%20%28double-precision%29) (TriggeredSeconds :type Float%20%28double-precision%29) (InputAction :type Input%20Action%20Object%20Reference :default "/Game/VehicleTemplate/Input/Actions/IA_Headlights.IA_Headlights"))
  ;[0.15 0.15 0.15 0.5] Input Management for Vehicle Pawn
  (bind _isa (Utilities|FlowControl|FlipFlop)
    (:A
      _)
    (:B
      _))
  (Rendering|SetVisibility (Variables|Default|GetHeadlight_L) _isa false))

(event EventPrimaryThumbstick
  (params (Axis :type Vector%202D%20Structure))
  ;[0.15 0.15 0.15 0.5] Input Management for Vehicle Pawn
  (Class|MetalCarsPawn|DoSteering (.x Axis))
  (if (>= (.y Axis) 0.0)
    (Class|MetalCarsPawn|DoThrottle (.y Axis))
    (if (Variables|Controls|GetBraking)
      (Variables|Controls|SetBraking false)
      (Class|MetalCarsPawn|DoBrakeStop))
    (else
      (Class|MetalCarsPawn|DoBrake (* (.y Axis) -1.0))
      (if (not (Variables|Controls|GetBraking))
        (Variables|Controls|SetBraking true)
        (Class|MetalCarsPawn|DoBrakeStart)))))

(event EventBeginPlay
  (|CallParentFunction)
  (Utilities|Time|SetTimerbyEvent (delegate Custom|CheckVFX) 0.1 true))

(event EventSecondaryThumbstick
  (params (Axis :type Vector%202D%20Structure))
  ;[0.15 0.15 0.15 0.5] Input Management for Vehicle Pawn
  (Class|MetalCarsPawn|DoLookAround (.x Axis)))

(event EventTouchHandbrakeStart
  ;[0.15 0.15 0.15 0.5] Input Management for Vehicle Pawn
  (Class|MetalCarsPawn|DoHandbrakeStart))

(event EventTouchHandbrakeEnd
  ;[0.15 0.15 0.15 0.5] Input Management for Vehicle Pawn
  (Class|MetalCarsPawn|DoHandbrakeStop))

(event EventTouchReset
  ;[0.15 0.15 0.15 0.5] Input Management for Vehicle Pawn
  (Class|MetalCarsPawn|DoResetVehicle))

(event EventTouchToggleCamera
  ;[0.15 0.15 0.15 0.5] Input Management for Vehicle Pawn
  (Class|MetalCarsPawn|DoToggleCamera))

(event EventTouchHeadlights
  ;[0.15 0.15 0.15 0.5] Input Management for Vehicle Pawn
  (bind _isa (Utilities|FlowControl|FlipFlop)
    (:A
      _)
    (:B
      _))
  (Rendering|SetVisibility (Variables|Default|GetHeadlight_L) _isa false))

(fn ConstructionScript)